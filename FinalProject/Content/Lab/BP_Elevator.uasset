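; BP_Elevator is an interactable elevator whose lift rises to a destination and returns automatically after a delay.
; OnInteract starts the LiftControl timeline, which drives PlaceLift to lerp the lift's relative location from its BeginPlay position to the ElevatorDestination component.
; When the upward run finishes, it waits ReturnDelay and reverses the same timeline.
; The IsMovingUp flag stops the timeline's Finished event from triggering another return after the descent.
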(event Custom|LiftStart
  (Variables|Default|SetIsMovingUp true)
  (bind _liftpercentage (Timeline|LiftControl Play)
    (:Update
      (CallFunction|PlaceLift _liftpercentage))
    (:Finished
      (if (Variables|Default|GetIsMovingUp)
        ;[0.15 0.15 0.15 0.5] Lift has reached the top, we need to wait before returning it. also set bool back to false
        (Utilities|FlowControl|Delay (Variables|Default|GetReturnDelay))
        (Variables|Default|SetIsMovingUp false)
        (CallFunction|LiftReturn)))))

(event Custom|LiftReturn
  (bind _liftpercentage (Timeline|LiftControl Reverse)
    (:Update
      (CallFunction|PlaceLift _liftpercentage))
    (:Finished
      (if (Variables|Default|GetIsMovingUp)
        ;[0.15 0.15 0.15 0.5] Lift has reached the top, we need to wait before returning it. also set bool back to false
        (Utilities|FlowControl|Delay (Variables|Default|GetReturnDelay))
        (Variables|Default|SetIsMovingUp false)
        (CallFunction|LiftReturn)))))

(event EventBeginPlay
  (Variables|Default|SetLiftStartLocation (Variables|/Script/Engine.SceneComponent|GetRelativeLocation (Variables|Default|GetElevatorLift))))

(fn ConstructionScript
  (|CallParentFunction))

(fn PlaceLift
  (params (Percent :type Float%20%28double-precision%29))
  (Transformation|SetRelativeLocation (Variables|Default|GetElevatorLift) (Math|Vector|Lerp(Vector) (Variables|Default|GetLiftStartLocation) (Variables|/Script/Engine.SceneComponent|GetRelativeLocation (Variables|Default|GetElevatorDestination)) Percent) false false))

(fn OnInteract
  (CallFunction|LiftStart))