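; BP_SlideDoor is a two-panel sliding door that toggles open and closed through its OnInteract function.
; BeginPlay caches both panels' relative start locations, and IsOpen decides whether OnInteract plays or reverses a single Timeline.
; Each Timeline update calls DoorSlideFunction per panel, offsetting them in opposite local Y directions by the square of the Percent track, preserving rotation and scale.
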(event Custom|OpenDoor
  (Variables|Default|SetIsOpen true)
  (bind _percent (Timeline|Timeline Play)
    (:Update
      (CallFunction|DoorSlideFunction (Variables|Default|GetDoorA) (Variables|Default|GetDoorAStartLocation) -1 _percent)
      (CallFunction|DoorSlideFunction (Variables|Default|GetDoorb) (Variables|Default|GetDoorBStartLocation) 1 _percent))))

(event Custom|CloseDoor
  (bind _percent (Timeline|Timeline Reverse)
    (:Update
      (CallFunction|DoorSlideFunction (Variables|Default|GetDoorA) (Variables|Default|GetDoorAStartLocation) -1 _percent)
      (CallFunction|DoorSlideFunction (Variables|Default|GetDoorb) (Variables|Default|GetDoorBStartLocation) 1 _percent))))

(event EventBeginPlay
  (Variables|Default|SetDoorAStartLocation (.location (Transformation|GetRelativeTransform (Variables|Default|GetDoorA))))
  (Variables|Default|SetDoorBStartLocation (.location (Transformation|GetRelativeTransform (Variables|Default|GetDoorb)))))

(fn ConstructionScript)

(fn DoorSlideFunction
  (params (DoorMesh :type Static%20Mesh%20Component%20Object%20Reference) (DoorStartingLocation :type Vector) (SlideDirection :type Integer) (Percent :type Float%20%28double-precision%29))
  (bind _returnvalue (Transformation|GetRelativeTransform DoorMesh))
  (Transformation|SetRelativeTransform DoorMesh (Math|Transform|MakeTransform (+ DoorStartingLocation (Math|Vector|MakeVector 0.0 (* SlideDirection Percent (Variables|Default|Getpercent)) 0.0)) (.rotation _returnvalue) (.scale _returnvalue)) false false))

(fn OnInteract
  (if (Variables|Default|GetIsOpen)
    (CallFunction|CloseDoor)
    (Variables|Default|SetIsOpen false)
    (else
      (CallFunction|OpenDoor)
      (Variables|Default|SetIsOpen true))))